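; BP_Computer is a clickable computer that opens a shopping menu when the top-down character reaches it.
; Hover swaps its material, and a click activates it so the next trigger overlap by the character starts the sequence.
; The character is hidden behind a posed stand-in mesh while the camera blends to the computer and the menu receives a spawn location.
; A delay loop polls for menu closure, then restores view, meshes and input and deactivates the object.
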(event `self.InteractableOBJ.OnBeginCursorOver`
  (params (TouchedComponent :type "PrimitiveComponent Object Reference"))
  (`PrimitiveComponent.SetMaterial` (`self.InteractableOBJ`) 0 (`self.Material`)))

(event `self.InteractableOBJ.OnEndCursorOver`
  (params (TouchedComponent :type "PrimitiveComponent Object Reference"))
  (`PrimitiveComponent.SetMaterial` (`self.InteractableOBJ`) 0 (`self.OverlapMaterial`)))

(event `self.InteractableOBJ.OnClicked`
  (params (TouchedComponent :type "PrimitiveComponent Object Reference") (ButtonPressed :type "Key Structure"))
  (`ActorComponent.Activate` (`self.InteractableOBJ`) false))

(event `self.Trigger.OnComponentBeginOverlap`
  (params (OverlappedComponent :type "PrimitiveComponent Object Reference") (OtherActor :type "Actor Object Reference") (OtherComp :type "PrimitiveComponent Object Reference") (OtherBodyIndex :type Integer) (bFromSweep :type Boolean) (SweepResult :type "HitResult Structure (by ref)"))
  (bind _returnvalue (`GameplayStatics.GetPlayerController` 0))
  (if (`ActorComponent.IsActive` (`self.InteractableOBJ`))
    (bind _asbp_top_down_character (cast `/Game/TopDown/Blueprints/BP_TopDownCharacter` OtherActor))
    (set `self.CharRef` _asbp_top_down_character)
    (`/Engine/EditorBlueprintResources/StandardMacros.DoOnce` false :!label _label
      (:`Completed`
        (`SkeletalMeshComponent.PlayAnimation` (`self.SkeletalMesh`) "/Game/Characters/Mannequins/Animations/Manny/MM_T_Pose.MM_T_Pose" false)
        (`WidgetBlueprintLibrary.SetInputMode_UIOnlyEx` (`GameplayStatics.GetPlayerController` 0) null)
        (`SceneComponent.SetVisibility` (`self.SkeletalMesh`) true false)
        (bind _mesh (`Character.Mesh` _asbp_top_down_character))
        (`SceneComponent.SetVisibility` _mesh false false)
        (`PlayerController.SetViewTargetWithBlend` _returnvalue self 1.0 "VTBlend_EaseInOut" 1.0 false)
        (bind _returnvalue_2 (`|CreateWidget` "/Game/UI/WDG_ShoppingMenu.WDG_ShoppingMenu_C" _returnvalue))
        (set `/Game/UI/WDG_ShoppingMenu.Spawn Transform` (`KismetMathLibrary.Conv_VectorToTransform` (`self.K2_GetActorLocation` (`self.Spawn Transform`))) _returnvalue_2)
        (bind _output_get (set `self.Widget` _returnvalue_2))
        (`UserWidget.AddToViewport` _output_get 0)
        (`KismetSystemLibrary.Delay` 2.0)
        (if (`/Game/UI/WDG_ShoppingMenu.MenuClosed` (`self.Widget`)) :!label _label_2
          (`PlayerController.SetViewTargetWithBlend` (`GameplayStatics.GetPlayerController` 0) _asbp_top_down_character 1.0 "VTBlend_EaseInOut" 1.0 false)
          (`SceneComponent.SetVisibility` (`self.SkeletalMesh`) false false)
          (`SceneComponent.SetVisibility` _mesh true false)
          (`ActorComponent.Deactivate` (`self.InteractableOBJ`))
          (`WidgetBlueprintLibrary.SetInputMode_GameAndUIEx` (`GameplayStatics.GetPlayerController` 0) null "DoNotLock" false)
          (goto _label :!via `Reset`)
          (else
            (`KismetSystemLibrary.Delay` 0.1)
            (goto _label_2)))))))

(fn `UserConstructionScript`)