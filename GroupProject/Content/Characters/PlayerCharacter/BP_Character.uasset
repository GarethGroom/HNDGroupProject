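; Player character Blueprint with spring-arm camera, single-item carrying and the level win check.
; On BeginPlay it sets Goal from the count of "Interactable" actors and shows the player UI and cursor.
; Scroll zooms; right-click turns the camera 90 degrees toward the cursor's screen half, eased on Tick.
; IA_PickUp attaches or drops "Pickupable" actors; Score equalling Goal shows game over, then opens the main menu.
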(event `Key|MouseScrollUp`
  (params (Key :type "Key Structure"))
  (bind _cameraboom (`self.CameraBoom`))
  ;[1 1 1] Camera zoom with scroll wheel
  (:`Pressed`
    (set `SpringArmComponent.TargetArmLength` (+ (`SpringArmComponent.TargetArmLength` _cameraboom) -100.0) _cameraboom)))

(event `Key|MouseScrollDown`
  (params (Key :type "Key Structure"))
  (bind _cameraboom (`self.CameraBoom`))
  ;[1 1 1] Camera zoom with scroll wheel
  (:`Pressed`
    (set `SpringArmComponent.TargetArmLength` (+ (`SpringArmComponent.TargetArmLength` _cameraboom) 100.0) _cameraboom)))

(event `self.ReceiveBeginPlay`
  (`|ExecutionSequence`
    (:`then_0`
      ;[1 1 1] Add all objects with tag ''Interactable' and add them to a int to set the goal
      (bind _outactors (`GameplayStatics.GetAllActorsWithTag` "Interactable"))
      (bind _output_get (set `self.AllInteractables` _outactors))
      (for _ _output_get
        (bind _result (`/Engine/EditorBlueprintResources/StandardMacros.IncrementInt` (`self.CounterOfInts`))
          (:`  `
            (set `self.CounterOfInts` _result))))
      (if (<= (`self.CounterOfInts`) 2)
        (bind _output_get_2 (set `self.Goal` 1))
        (`KismetSystemLibrary.PrintString` (`KismetStringLibrary.Conv_IntToString` _output_get_2))
        (else
          (bind _output_get_3 (set `self.Goal` (+ (/ (`self.CounterOfInts`) 2) 1)))
          (`KismetSystemLibrary.PrintString` (`KismetStringLibrary.Conv_IntToString` _output_get_3)))))
    (:`then_1`
      (bind _returnvalue (`|CreateWidget` "/Game/UI/WDG_PlayerUI.WDG_PlayerUI_C"))
      (`UserWidget.AddToViewport` _returnvalue 0)
      (set `PlayerController.bShowMouseCursor` true (`GameplayStatics.GetPlayerController` 0)))))

(event `LevelComplete`
  ;[1 1 1] On level complete return to main menu
  (bind _returnvalue (`|CreateWidget` "/Game/UI/WDG_GameOver.WDG_GameOver_C"))
  (`UserWidget.AddToViewport` _returnvalue 0)
  (`KismetSystemLibrary.Delay` 5.0)
  (`GameplayStatics.OpenLevel` "LvL_MainMenu"))

(event `EnhancedInput|/Game/TopDown/Input/Actions/IA_PickUp`
  (params (ActionValue :type Boolean) (ElapsedSeconds :type "Float (double-precision)") (TriggeredSeconds :type "Float (double-precision)") (InputAction :type "InputAction Object Reference" :default "/Game/TopDown/Input/Actions/IA_PickUp.IA_PickUp"))
  ;[1 1 1] Pickup and drop item
  (:`Completed`
    (if (`self.IsHolding?`)
      ;;[1 1 1] Drop Item
      (`self.K2_DetachFromActor` (`self.HeldItem`) "KeepWorld" "KeepWorld" "KeepWorld")
      (set `self.IsHolding?` false)
      (else
        ;;[1 1 1] Pickup item
        (for _array_element (`self.GetOverlappingActors` "/Script/Engine.Actor")
          (if (`self.ActorHasTag` _array_element "Pickupable")
            (bind _output_get (set `self.HeldItem` _array_element))
            (`self.K2_AttachToComponent` _output_get (`self.Mesh`) "ItemSocket" "SnapToTarget" "SnapToTarget" "KeepRelative" true)
            (set `self.IsHolding?` true)
            (`KismetSystemLibrary.PrintString` "Item Grabbed")))))))

(event `Key|RightMouseButton`
  (params (Key :type "Key Structure"))
  (bind (_desiredyawrotation_roll _desiredyawrotation_pitch _desiredyawrotation_yaw) (`KismetMathLibrary.BreakRotator` (`self.DesiredYawRotation`)))
  (:`Pressed`
    (set `self.DesiredYawRotation` (`KismetMathLibrary.MakeRotator` _desiredyawrotation_roll _desiredyawrotation_pitch (+ _desiredyawrotation_yaw (* (stale `self.ReceiveTick` _value) 90.0))))))

(event `self.ReceiveTick`
  (params (DeltaSeconds :type "Float (single-precision)"))
  (`|ExecutionSequence`
    (:`then_0`
      (bind _value (`self.GetPointerXValue`)))
    (:`then_1`
      (`self.UpdateCameraYaw`))
    (:`then_2`
      (if (== (`self.Score`) (`self.Goal`))
        (`self.LevelComplete`)))))

(fn `GetPointerXValue`
  (returns (Value :type "Float (double-precision)"))
  (bind _returnvalue_x (`KismetMathLibrary.BreakVector2D` (`WidgetLayoutLibrary.GetViewportSize`)))
  (return (`KismetMathLibrary.SelectFloat` -1.0 1.0 (< (`PlayerController.GetMousePosition` (`GameplayStatics.GetPlayerController` 0)) (/ _returnvalue_x 2.0)))))

(fn `UpdateCameraYaw`
  (`SceneComponent.K2_SetRelativeRotation` (`self.CameraBoom`) (`KismetMathLibrary.RInterpTo` (`SceneComponent.RelativeRotation` (`self.CameraBoom`)) (`self.DesiredYawRotation`) (`GameplayStatics.GetWorldDeltaSeconds`) 3.0) false false))

(fn `UserConstructionScript`)